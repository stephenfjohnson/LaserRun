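; BP_FloorButton is a floor button that activates linked objects while pressed.
; A sphere overlap plays a timeline lowering the button and sends ActivateMessage through BPI_Activatable to ActivateObjects; its player/physics check gates nothing visible.
; When the first-person character or a physics-simulating component leaves and neither remains overlapping, it reverses the timeline and sends DeactivateMessage.
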(event OnComponentBeginOverlap(ColSphere)
  (params (OverlappedComponent :type Primitive%20Component%20Object%20Reference) (OtherActor :type Actor%20Object%20Reference) (OtherComp :type Primitive%20Component%20Object%20Reference) (OtherBodyIndex :type Integer) (bFromSweep :type Boolean) (SweepResult :type Hit%20Result%20Structure%20%28by%20ref%29))
  (CallFunction|CheckforPhysicsSimOverlap OtherActor OtherComp)
  (CallFunction|DownAnimation)
  (for _array_element (Variables|Default|GetActivateObjects)
    (if (Utilities|DoesObjectImplementInterface _array_element "/Game/Blueprints/BPI_Activatable.BPI_Activatable_C")
      (Class|BPIActivatable|Activate(Message) _array_element))))

(event OnComponentEndOverlap(ColSphere)
  (params (OverlappedComponent :type Primitive%20Component%20Object%20Reference) (OtherActor :type Actor%20Object%20Reference) (OtherComp :type Primitive%20Component%20Object%20Reference) (OtherBodyIndex :type Integer))
  (if (and (or (== (Utilities|GetClass OtherActor) "/Game/Blueprints/BP_FirstPersonCharacter.BP_FirstPersonCharacter_C") (Physics|IsSimulatingPhysics OtherComp "None")) (CallFunction|AreThereNotAnyObjectsonTopOfButton))
    (CallFunction|UpAnimation)
    (for _array_element (Variables|Default|GetActivateObjects)
      (if (Utilities|DoesObjectImplementInterface _array_element "/Game/Blueprints/BPI_Activatable.BPI_Activatable_C")
        (Class|BPIActivatable|Deactivate(Message) _array_element)))))

(event Custom|DownAnimation
  (bind _zoffset (Timeline|ButtonDown Play)
    (:Update
      (Transformation|SetRelativeLocation (Variables|Default|GetButton) (Math|Vector|MakeVector 0.0 0.0 _zoffset) false false))))

(event Custom|UpAnimation
  (bind _zoffset (Timeline|ButtonDown Reverse)
    (:Update
      (Transformation|SetRelativeLocation (Variables|Default|GetButton) (Math|Vector|MakeVector 0.0 0.0 _zoffset) false false))))

(event EventBeginPlay)

(event Collision|EventActorBeginOverlap
  (params (OtherActor :type Actor%20Object%20Reference)))

(event EventTick
  (params (DeltaSeconds :type Float%20%28single-precision%29)))

(fn ConstructionScript)

(fn CheckforPhysicsSimOverlap
  (params (FirstPerson :type Object%20Object%20Reference) (PhysicsObjects :type Scene%20Component%20Object%20Reference))
  (if (or (== (Utilities|GetClass FirstPerson) "/Game/Blueprints/BP_FirstPersonCharacter.BP_FirstPersonCharacter_C") (Physics|IsSimulatingPhysics PhysicsObjects "None"))
    _))

(fn AreThereNotAnyObjectsonTopOfButton
  (LocalVariables|SetIsObjectOnButton false)
  (for _array_element (Class|PrimitiveComponent|GetOverlappingComponents (Variables|Default|GetColSphere))
    (if (Physics|IsSimulatingPhysics _array_element "None")
      (LocalVariables|SetIsObjectOnButton true)))
  (return (and (not (LocalVariables|GetIsObjectOnButton)) (== (Utilities|Array|Length (Collision|GetOverlappingActors (Variables|Default|GetColSphere) "/Game/Blueprints/BP_FirstPersonCharacter.BP_FirstPersonCharacter_C" :!class /Script/Engine.PrimitiveComponent)) 0))))