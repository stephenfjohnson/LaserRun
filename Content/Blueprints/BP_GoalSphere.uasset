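; BP_GoalSphere is a goal sphere actor that switches a set of linked objects on and off.
; StartActivation and EndActivation flip an IsActivated flag, which guards against repeated triggers.
; On each change it loops through ActivateObjects and sends ActivateMessage or DeactivateMessage to those implementing BPI_Activatable.
; The file does not include what calls the two events.
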(event Custom|StartActivation
  (if (not (Variables|Default|GetIsActivated?))
    (Variables|Default|SetIsActivated? true)
    (for _array_element (Variables|Default|GetActivateObjects)
      (if (Utilities|DoesObjectImplementInterface _array_element "/Game/Blueprints/BPI_Activatable.BPI_Activatable_C")
        (Class|BPIActivatable|Activate(Message) _array_element)))))

(event Custom|EndActivation
  (if (Variables|Default|GetIsActivated?)
    (Variables|Default|SetIsActivated? false)
    (for _array_element (Variables|Default|GetActivateObjects)
      (if (Utilities|DoesObjectImplementInterface _array_element "/Game/Blueprints/BPI_Activatable.BPI_Activatable_C")
        (Class|BPIActivatable|Deactivate(Message) _array_element)))))

(fn ConstructionScript)